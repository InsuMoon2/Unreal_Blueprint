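; BP_Helpers provides a helper that picks the actor from an array lying closest to a character's view direction.
; It dots the flattened 2D direction to each actor with the forward vector of the character's control rotation.
; The highest dot product at or above the running Angle value wins, so Angle holds a cosine and distance plays no part.
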(fn GetNearlyFrontAngle
  (params (InCharacter :type Character%20Object%20Reference) (InArray :type Array%20of%20Character%20Object%20References))
  (for _array_element InArray
    (if (>= (Math|Vector|DotProduct (Class|KismetMathLibrary|VectorNormal2D (- (Transformation|GetActorLocation _array_element) (Transformation|GetActorLocation InCharacter)) 0.0001) (Math|Vector|GetForwardVector (Pawn|GetControlRotation InCharacter :!class /Script/Engine.Pawn))) (LocalVariables|GetAngle))
      (LocalVariables|SetAngle (Math|Vector|DotProduct (Class|KismetMathLibrary|VectorNormal2D (- (Transformation|GetActorLocation _array_element) (Transformation|GetActorLocation InCharacter)) 0.0001) (Math|Vector|GetForwardVector (Pawn|GetControlRotation InCharacter :!class /Script/Engine.Pawn))))
      (LocalVariables|SetCandidate _array_element)))
  (return (LocalVariables|GetCandidate)))
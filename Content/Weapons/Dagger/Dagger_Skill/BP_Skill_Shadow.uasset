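; Afterimage actor for the dagger's shadow skill that leaves a fading, posed copy of player 0's character.
; On BeginPlay its PoseableMesh takes the player's skeletal mesh, then a loop applies the trail material to the first seven slots and copies the current pose.
; A timeline, restarted within that loop, drives the "Opercity" material parameter and destroys the actor when it finishes.
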(event EventBeginPlay
  (bind _returnvalue (Game|GetPlayerCharacter 0))
  (bind _poseablemesh (Variables|Default|GetPoseableMesh))
  (bind _poseablemesh_2 (Variables|Default|GetPoseableMesh))
  (bind _mesh (Variables|/Script/Engine.Character|GetMesh _returnvalue))
  (Class|SkinnedMeshComponent|SetSkeletalMesh _poseablemesh_2 (Variables|/Script/Engine.SkinnedMeshComponent|GetSkeletalMesh _mesh) true)
  (for _index (range 0 6)
    (Rendering|Material|SetMaterial _poseablemesh_2 _index "/Game/Materials/M_Trail_Inst.M_Trail_Inst")
    (Class|PoseableMeshComponent|CopyPosefromSkeletalComponent _poseablemesh _mesh)
    (bind _새_트랙_0 (Timeline|타임라인_0 PlayFromStart)
      (:Update
        (Rendering|Material|SetScalarParameterValueonMaterials _poseablemesh "Opercity" _새_트랙_0))
      (:Finished
        (Actor|DestroyActor)))))

(fn ConstructionScript)
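; BP_Enemy_Basic is a basic AI enemy that links its state component to its Blackboard behavior and hides its sheath bone on BeginPlay.
; A state-change binding writes the hit behavior enum to the Blackboard "Behavior" key whenever the enemy enters Hitted, Air Hitted or Skill Hitted.
; Each tick it reads that key back and displays the enum name on the Behavior text.
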(event Custom|OnStateTypeChanged_AI
  (params (InPrevType :type EStateType%20Enum :default "NewEnumerator0") (InNewType :type EStateType%20Enum :default "NewEnumerator0"))
  (bind (_target _enemy_behavior _hitted) (|N_Hitted))
  (switch Utilities|FlowControl|Switch|SwitchonEStateType InNewType
    (:NewEnumerator5
      _)
    (:NewEnumerator8
      _)
    (:NewEnumerator15
      _))
  (AI|Components|Blackboard|SetValueasEnum _target _enemy_behavior _hitted))

(event EventBeginPlay
  (|CallParentFunction)
  (Utilities|FlowControl|Sequence
    (:then_0
      (Components|SkinnedMesh|HideBonebyName (Variables|Character|GetMesh) "cc_sheath_00" "PBO_None"))
    (:then_1
      (EventDispatchers|BindEventtoOnStateTypeChanged (Variables|Default|GetStateComponent) (delegate Custom|OnStateTypeChanged_AI)))))

(event EventTick
  (params (DeltaSeconds :type Float%20%28single-precision%29))
  (|CallParentFunction 0.0)
  (Rendering|Components|TextRender|SetText (Variables|Default|GetBehavior) (Utilities|Text|ToText(String) (Utilities|String|EnumtoString (Utilities|Enum|ByteToEnumEEnemy_Basic_BehaviorType (Class|BlackboardComponent|GetValueasEnum (AI|GetBlackboard (AI|GetAIController self)) (Utilities|Name|MakeLiteralName "Behavior")))))))

(fn ConstructionScript
  (|CallParentFunction))
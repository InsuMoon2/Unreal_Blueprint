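; BP_Boss_Sion_Child is a child variant of the Sion boss enemy with its own max health, a name-and-health bar and a hidden boss HP widget.
; Normal, upper and skill damage events call the parent, set the matching hit mode on StateComponent, then trigger their hit reaction.
; Normal and skill hits enter a collapsed health-check graph leading to BeginDead, but its decrement logic is unwired.
; The stun montage graph is also unwired.
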(event EventBeginPlay
  (|CallParentFunction)
  (Utilities|FlowControl|Sequence
    (:then_0
      (Variables|Default|SetHealth (Variables|Default|GetMax_Health_Child))
      (CallFunction|UpdateHealthBar))
    (:then_1
      (Widget|SetVisibility (Variables|Default|GetBoss_HpWidget) "Hidden"))))

(event EventDamaged
  (params (Attacker :type Character%20Object%20Reference) (Causer :type Actor%20Object%20Reference) (HitData :type F%20Hit%20Data%20Structure) (BackAttack :type Anim%20Montage%20Object%20Reference))
  ;[1 1 1] Damaged
  (|CallParentFunction Attacker Causer HitData BackAttack)
  (Default|SetHittedMode (Variables|Default|GetStateComponent))
  (CallFunction|Hitted))

(event EventSkillDamaged
  (params (Attacker :type Character%20Object%20Reference) (Causer :type Actor%20Object%20Reference) (SkillHitData :type F%20Skill%20Hit%20Data%20Structure))
  ;[1 1 1] Damaged
  (|CallParentFunction Attacker Causer SkillHitData)
  (Default|SetSkillHittedMode (Variables|Default|GetStateComponent))
  (CallFunction|SkillHitted))

(event EventHitted
  ;[1 1 1] Damaged
  (|CallParentFunction)
  (|CollapseGraph_0
    (:True
      (CallFunction|BeginDead))))

(event EventUpperDamaged
  (params (Attacker :type Character%20Object%20Reference) (Causer :type Actor%20Object%20Reference) (UpperHitData :type F%20Air%20Hit%20Data%20Structure))
  ;[1 1 1] Damaged
  (|CallParentFunction Attacker Causer UpperHitData)
  (Default|SetAirHittedMode (Variables|Default|GetStateComponent))
  (CallFunction|AirComboHitted))

(event EventAirComboHitted
  ;[1 1 1] Damaged
  (|CallParentFunction))

(event EventSkillHitted
  ;[1 1 1] Damaged
  (|CallParentFunction)
  (|CollapseGraph_0
    (:True
      (CallFunction|BeginDead))))

(fn ConstructionScript
  (|CallParentFunction))

(fn UpdateHealthBar
  (|CallParentFunction)
  (bind _aswb_name (Utilities|Casting|CastToWB_Name (UserInterface|GetUserWidgetObject (Variables|Default|GetHealthBar))))
  (Default|UpdateHealth _aswb_name (Variables|Default|GetHealth) (Variables|Default|GetMax_Health_Child))
  (Default|UpdateName _aswb_name (Utilities|GetDisplayName self)))
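; Boss enemy Sion, which equips a sword, shows an HP widget and takes normal, air and skill hits.
; Each hit drains shield first, otherwise health and lethargy; zero health triggers death, while broken shield or empty lethargy triggers stun and updates the AI blackboard.
; Hit data drives particles and sound, plus camera shake for normal hits; knockback, turn-to-attacker and hit-stop are unwired.
; Tick refreshes debug state text and the shield bar.
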(event Custom|AirCombo_Hitted
  (bind (_target _enemy_behavior _hitted) (|Set_Hitted_2))
  ;[1 1 1] Damaged, Hitted
  (|SetAir_Damage (.Damage (Utilities|Struct|BreakFAirHitData (Variables|HitData|GetAirHitData)))
    (:Dead
      (CallFunction|BeginDead))
    (:Hitted
      (|ApplyAir_Damage))
    (:Lethargy
      (CallFunction|BeginLethargy :!label _label)
      (AI|Components|Blackboard|SetValueasEnum _target _enemy_behavior _hitted)
      (Default|CallOnDestructibleCollisionType))
    (:Shield
      (goto _label))))

(event Custom|Skill_Hitted
  (bind (_target _enemy_behavior _hitted) (|Set_Hitted_2))
  ;[1 1 1] Damaged, Hitted
  (|SetSkill_Damage (.Damage (Utilities|Struct|BreakFSkillHitData (Variables|HitData|GetSkillHitData)))
    (:Dead
      (CallFunction|BeginDead))
    (:Hitted
      (|ApplySkill_Damage))
    (:Lethargy
      (CallFunction|BeginLethargy :!label _label)
      (AI|Components|Blackboard|SetValueasEnum _target _enemy_behavior _hitted)
      (Default|CallOnDestructibleCollisionType))
    (:Shield
      (goto _label))))

(event Custom|End_Dead
  ;[1 1 1] Dead
  (Actor|DestroyActor))

(event Custom|Hitted
  (bind (_target _enemy_behavior _hitted) (|Set_Hitted_2))
  ;[1 1 1] Damaged, Hitted
  (|SetDamage (.Damage (Utilities|Struct|BreakFHitData (Variables|HitData|GetHitData)))
    (:Dead
      (CallFunction|BeginDead))
    (:Hitted
      (Game|Damage|ApplyDamage))
    (:Lethargy
      (CallFunction|BeginLethargy :!label _label)
      (AI|Components|Blackboard|SetValueasEnum _target _enemy_behavior _hitted)
      (Default|CallOnDestructibleCollisionType))
    (:Shield
      (goto _label))))

(event Custom|Begin_Dead
  ;[1 1 1] Dead
  (Collision|SetCollisionEnabled (Variables|Default|GetCapsuleComponent) "NoCollision")
  (Animation|PlayAnimMontage "/Game/Enemies/Sion/Animation/Sion_Death.Sion_Death" 1.0 "None")
  (Default|Stop (Variables|Default|GetMovingComponent)))

(event Custom|Begin_Lethargy
  ;[1 1 1] Dead
  (if (not (Default|IsStunMode (Variables|Default|GetStateComponent)))
    (Default|SetStunMode (Variables|Default|GetStateComponent))
    (Default|Stop (Variables|Default|GetMovingComponent))
    (Animation|PlayAnimMontage "/Game/Enemies/Sion/Animation/Sion_Stun_Lethargy.Sion_Stun_Lethargy" 1.0 "None")))

(event Custom|End_Lethargy
  ;[1 1 1] Dead
)

(event EventDamaged
  (params (Attacker :type Character%20Object%20Reference) (Causer :type Actor%20Object%20Reference) (HitData :type F%20Hit%20Data%20Structure) (BackAttack :type Anim%20Montage%20Object%20Reference))
  ;[1 1 1] Damaged, Hitted
  (Variables|Default|SetAttacker Attacker)
  (Variables|Default|SetCauser Causer)
  (Variables|HitData|SetHitData HitData)
  (Variables|Default|SetBackAttack_Montage BackAttack)
  (CallFunction|Hitted))

(event EventUpperDamaged
  (params (Attacker :type Character%20Object%20Reference) (Causer :type Actor%20Object%20Reference) (UpperHitData :type F%20Air%20Hit%20Data%20Structure))
  ;[1 1 1] Damaged, Hitted
  (Variables|Default|SetAttacker Attacker)
  (Variables|Default|SetCauser Causer)
  (Variables|HitData|SetAirHitData UpperHitData)
  (CallFunction|AirComboHitted))

(event EventBeginPlay
  (Utilities|FlowControl|Sequence
    (:then_0
      (|SettingValue :!label _label))
    (:then_1
      (goto _label execute2))
    (:then_2
      (goto _label execute3))
    (:then_3
      (goto _label execute4))
    (:then_4
      (|Setting_Value2 :!label _label_2))
    (:then_5
      (goto _label_2 execute2))))

(event EventSkillDamaged
  (params (Attacker :type Character%20Object%20Reference) (Causer :type Actor%20Object%20Reference) (SkillHitData :type F%20Skill%20Hit%20Data%20Structure))
  ;[1 1 1] Damaged, Hitted
  (Variables|Default|SetAttacker Attacker)
  (Variables|Default|SetCauser Causer)
  (Variables|HitData|SetSkillHitData SkillHitData)
  (CallFunction|SkillHitted))

(event EventTick
  (params (DeltaSeconds :type Float%20%28single-precision%29))
  (|CallParentFunction DeltaSeconds)
  (Utilities|FlowControl|Sequence
    (:then_0
      (|Enemy_State))
    (:then_1
      (CallFunction|UpdateShieldBar))))

(fn ConstructionScript)

(fn UpdateHealthBar
  (bind _boss_hpwidget (Variables|Default|GetBoss_HpWidget))
  (Utilities|IsValid _boss_hpwidget
    (:Is%20Valid
      (Default|UpdateHealth _boss_hpwidget (Variables|Default|GetHealth) (Variables|Default|GetMaxHealth)))))

(fn UpdateLethargyBar
  (bind _boss_hpwidget (Variables|Default|GetBoss_HpWidget))
  (Utilities|IsValid _boss_hpwidget
    (:Is%20Valid
      (Default|UpdateLethargy _boss_hpwidget (Variables|Default|GetLethargy) (Variables|Default|GetMaxLethargy)))))

(fn CrossHairon
  (Rendering|SetVisibility (Variables|Default|GetCrossHair) true false))

(fn CrossHairOff
  (Rendering|SetVisibility (Variables|Default|GetCrossHair) false false))

(fn IsCrossHairVisible
  (return (Rendering|IsVisible (Variables|Default|GetCrossHair))))

(fn SetInitLethargy
  (Variables|Default|SetLethargy (Variables|Default|GetMaxLethargy))
  (CallFunction|UpdateLethargyBar))

(fn GetSkillIndex
  (return (Variables|Default|GetSkill_Index)))

(fn UpdateShieldBar
  (bind _boss_hpwidget (Variables|Default|GetBoss_HpWidget))
  (Utilities|IsValid _boss_hpwidget
    (:Is%20Valid
      (Default|UpdateShield _boss_hpwidget (Variables|Default|GetShield) (Variables|Default|GetMaxShield)))))

(fn IsZeroShield
  (return (<= (Variables|Default|GetShield) 0.001)))

(event Custom|OnStateTypeChanged
  (params (InPrevType :type EStateType%20Enum :default "NewEnumerator0") (InNewType :type EStateType%20Enum :default "NewEnumerator0"))
  (switch Utilities|FlowControl|Switch|SwitchonEStateType InNewType
    (:NewEnumerator5
      (CallFunction|Hitted))
    (:NewEnumerator8
      (CallFunction|AirComboHitted))
    (:NewEnumerator15
      (CallFunction|SkillHitted))))

(event Custom|RestoreTimeDelation
  (bind _delationactors (Variables|Default|GetDelationActors))
  (for _array_element _delationactors
    (Variables|/Script/Engine.Actor|SetCustomTimeDilation _array_element 1.0))
  (Utilities|Array|Clear _delationactors))
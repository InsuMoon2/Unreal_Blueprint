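; AI controller for the Shadow Dagger pawn, which targets enemy AI and the Sion boss.
; On possess it caches the pawn and runs the behavior tree stored on it.
; Each perception update writes the first perceived BP_Enemy_AI or BP_Boss_Sion to the blackboard's Target key, clearing the key when none is found.
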(event OnPerceptionUpdated(AIPerception)
  (params (UpdatedActors :type Array%20of%20Actor%20Object%20References))
  (CallFunction|Perception))

(event EventPossess
  (params (PossessedPawn :type Pawn%20Object%20Reference))
  (bind _asbp_shadow_dagger (Utilities|Casting|CastToBP_Shadow_Dagger PossessedPawn))
  (bind _output_get (Variables|Default|SetShadow_Dagger_AI _asbp_shadow_dagger))
  (AI|RunBehaviorTree (Variables|/Game/Enemies/Shadow/BP_Shadow_Dagger.BP_Shadow_Dagger_C|GetBehaviorTree _output_get)))

(fn ConstructionScript)

(fn Perception
  (for _array_element (Class|AIPerceptionComponent|GetCurrentlyPerceivedActors (Variables|Default|GetAIPerception))
    (bind _asbp_enemy_ai (Utilities|Casting|CastToBP_Enemy_AI _array_element)
      (:then
        (AI|Components|Blackboard|SetValueasObject (AI|GetBlackboard 0) (Utilities|Name|MakeLiteralName "Target") _asbp_enemy_ai))
      (:CastFailed
        (bind _asbp_boss_sion (Utilities|Casting|CastToBP_Boss_Sion _array_element))
        (AI|Components|Blackboard|SetValueasObject (AI|GetBlackboard 0) (Utilities|Name|MakeLiteralName "Target") _asbp_boss_sion)))
    (return))
  (AI|Components|Blackboard|SetValueasObject (AI|GetBlackboard 0) (Utilities|Name|MakeLiteralName "Target") 0))
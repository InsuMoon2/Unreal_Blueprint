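; BP_Shadow_Dagger is a short-lived, dagger-wielding "Shadow" AI character that destroys itself after about 15 seconds.
; On BeginPlay it fills health, binds state changes, equips daggers with a trail material and hides its state widget.
; Hit and skill states write the blackboard Behavior enum, death calls BeginDead, and hits refresh the health bar.
; Tick keeps SkillCost pinned, shows the current behavior as text and counts the lifetime.
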(event EventHitted
  (|CallParentFunction)
  (CallFunction|UpdateWidget))

(event EventBeginPlay
  (|CallParentFunction)
  (Utilities|FlowControl|Sequence
    (:then_0
      (|Setting :!label _label))
    (:then_1
      (goto _label execute))
    (:then_2
      (goto _label execute2))
    (:then_3
      (goto _label execute3))
    (:then_4
      (goto _label execute4))))

(event EventTick
  (params (DeltaSeconds :type Float%20%28single-precision%29))
  (|CallParentFunction DeltaSeconds)
  (Utilities|FlowControl|Sequence
    (:then_0
      (Rendering|Components|TextRender|SetText))
    (:then_1
      (Variables|Default|SetSkillCost 1e+02))
    (:then_2
      (bind _output_get (Variables|Default|SetSpawnTime (+ DeltaSeconds (Variables|Default|GetSpawnTime)))))
    (:then_3
      ;[1 1 1] Dead
      (if (> (Variables|Default|GetSpawnTime) 15.0)
        (Actor|DestroyActor)))))

(event EventSkillHitted
  (|CallParentFunction)
  (CallFunction|UpdateWidget))

(fn ConstructionScript
  (|CallParentFunction))

(fn UpdateWidget
  (bind _aswb_name (Utilities|Casting|CastToWB_Name (UserInterface|GetUserWidgetObject (Variables|Default|GetHealthBar))))
  (Default|UpdateHealth _aswb_name (Variables|Default|GetHealth) (Variables|Default|GetMaxHealth))
  (Default|UpdateName _aswb_name "Shadow"))

(event Custom|OnStateTypeChanged_Shadow
  (params (InPrevType :type EStateType%20Enum :default "NewEnumerator0") (InNewType :type EStateType%20Enum :default "NewEnumerator0"))
  (bind (_returnvalue3 _returnvalue2 _returnvalue) (|N_Hitted))
  (bind (_returnvalue3_2 _returnvalue2_2 _returnvalue_2) (|N_Skill))
  (switch Utilities|FlowControl|Switch|SwitchonEStateType InNewType
    (:NewEnumerator5
      (AI|Components|Blackboard|SetValueasEnum _returnvalue3 _returnvalue2 _returnvalue))
    (:NewEnumerator7
      (CallFunction|BeginDead))
    (:NewEnumerator10
      (AI|Components|Blackboard|SetValueasEnum _returnvalue3_2 _returnvalue2_2 _returnvalue_2))))
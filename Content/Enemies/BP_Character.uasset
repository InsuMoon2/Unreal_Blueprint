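; BP_Character is a character Blueprint in the Enemies folder that carries a team index for telling allies from opponents.
; Simple setter and getter functions manage the index, and IsSameTeam checks that two given characters are valid before comparing their indices.
; Every Tick, the current index is written to TeamIndexText, keeping the displayed team number up to date.
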(event EventTick
  (params (DeltaSeconds :type Float%20%28single-precision%29))
  (Rendering|Components|TextRender|SetText (Variables|Default|GetTeam_Index_text) (Utilities|Text|ToText(Integer) (CallFunction|IsTeamIndex))))

(fn ConstructionScript)

(fn TeamIndex
  (params (InTeamIndex :type Integer))
  (Variables|Default|SetTeam_Index InTeamIndex)
  (return))

(fn IsTeamIndex
  (return (Variables|Default|GetTeam_Index)))

(fn IsSameTeam
  (params (InCharacter1 :type BP%20Character%20Object%20Reference) (InCharacter2 :type BP%20Character%20Object%20Reference))
  (Utilities|IsValid InCharacter1
    (:Is%20Valid
      (Utilities|IsValid InCharacter2
        (:Is%20Valid
          (return (== (CallFunction|IsTeamIndex InCharacter1) (CallFunction|IsTeamIndex InCharacter2))))))))
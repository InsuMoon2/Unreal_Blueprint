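; Ranged enemy AI Blueprint that keeps its behavior tree Blackboard in step with the enemy's combat state.
; On BeginPlay it binds to StateComponent type changes, writing one Behavior enum value for Idle and another shared by Hitted, Air Hitted and Skill Hitted.
; Tick shows the current Behavior as text, converting it through the Shield enemy's enum rather than the Range one.
; Hit events defer to the parent.
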(event Custom|OnStateTypeChanged_AI
  (params (InPrevType :type EStateType%20Enum :default "NewEnumerator0") (InNewType :type EStateType%20Enum :default "NewEnumerator0"))
  (bind (_target _enemy_behavior _hitted) (|N_Hitted_2_2))
  (bind (_target_2 _enemy_behavior_2 _hitted_2) (|N_Hitted_2))
  (switch Utilities|FlowControl|Switch|SwitchonEStateType InNewType
    (:NewEnumerator0
      (AI|Components|Blackboard|SetValueasEnum _target _enemy_behavior _hitted))
    (:NewEnumerator5
      (AI|Components|Blackboard|SetValueasEnum _target_2 _enemy_behavior_2 _hitted_2 :!label _label))
    (:NewEnumerator8
      (goto _label))
    (:NewEnumerator15
      (goto _label))))

(event EventBeginPlay
  (|CallParentFunction)
  (Utilities|FlowControl|Sequence
    (:then_0
      (EventDispatchers|BindEventtoOnStateTypeChanged (Variables|Default|GetStateComponent) (delegate Custom|OnStateTypeChanged_AI)))))

(event EventTick
  (params (DeltaSeconds :type Float%20%28single-precision%29))
  (|CallParentFunction DeltaSeconds)
  (Utilities|FlowControl|Sequence
    (:then_0
      (|Set_State_2))))

(event EventHitted
  (|CallParentFunction))

(event EventAirComboHitted
  (|CallParentFunction))

(event EventSkillHitted
  (|CallParentFunction))

(fn ConstructionScript
  (|CallParentFunction))
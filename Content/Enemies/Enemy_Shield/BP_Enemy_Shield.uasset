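; Shield enemy Blueprint that extends its parent's hit reactions and links character state to AI behavior.
; Hit events play a shield block montage when the equipped weapon is in guard.
; State component changes to hit or guard write behavior enums to the blackboard, with hits using the "Behavior" key and guard using "Enemy_Behavior".
; Each tick, the "Behavior" value is shown as text on the enemy.
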(event EventBeginPlay
  (|CallParentFunction)
  (Utilities|FlowControl|Sequence
    (:then_0
      (|Enemy_state))))

(event EventTick
  (params (DeltaSeconds :type Float%20%28single-precision%29))
  (|CallParentFunction DeltaSeconds)
  (Utilities|FlowControl|Sequence
    (:then_1
      (|Set_State))))

(event EventHitted
  (|CallParentFunction)
  (bind _weapon (Variables|/Game/Components/WeaponComponent.WeaponComponent_C|GetWeapon (Variables|Default|GetWeaponComponent))
    (:then
      (if (Variables|/Game/Weapons/Weapon.Weapon_C|GetInGuard _weapon)
        (Animation|PlayAnimMontage self "/Game/Enemies/Enemy_Shield/Montage/Shield_Guard_Block.Shield_Guard_Block" 0.8 "None")))
    (:else)))

(event EventAirComboHitted
  (|CallParentFunction)
  (bind _weapon (Variables|/Game/Components/WeaponComponent.WeaponComponent_C|GetWeapon (Variables|Default|GetWeaponComponent))
    (:then
      (if (Variables|/Game/Weapons/Weapon.Weapon_C|GetInGuard _weapon)
        (Animation|PlayAnimMontage self "/Game/Enemies/Enemy_Shield/Montage/Shield_Guard_Block.Shield_Guard_Block" 0.8 "None")))
    (:else)))

(event EventSkillHitted
  (|CallParentFunction)
  (bind _weapon (Variables|/Game/Components/WeaponComponent.WeaponComponent_C|GetWeapon (Variables|Default|GetWeaponComponent))
    (:then
      (if (Variables|/Game/Weapons/Weapon.Weapon_C|GetInGuard _weapon)
        (Animation|PlayAnimMontage self "/Game/Enemies/Enemy_Shield/Montage/Shield_Guard_Block.Shield_Guard_Block" 0.8 "None")))
    (:else)))

(fn ConstructionScript
  (|CallParentFunction))

(event Custom|OnStateTypeChanged_AI
  (params (InPrevType :type EStateType%20Enum :default "NewEnumerator0") (InNewType :type EStateType%20Enum :default "NewEnumerator0"))
  (bind (_target _enemy_behavior _hitted) (|N_Hitted))
  (bind (_target_2 _enemy_behavior_2 _hitted_2) (|N_Guard))
  (switch Utilities|FlowControl|Switch|SwitchonEStateType InNewType
    (:NewEnumerator5
      (AI|Components|Blackboard|SetValueasEnum _target _enemy_behavior _hitted :!label _label))
    (:NewEnumerator8
      (goto _label))
    (:NewEnumerator15
      (goto _label))
    (:NewEnumerator13
      (AI|Components|Blackboard|SetValueasEnum _target_2 _enemy_behavior_2 _hitted_2))))
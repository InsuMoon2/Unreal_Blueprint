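; AI controller for the shield enemy, giving it a behavior tree and a hostile target to act on.
; On possession it caches the BP_Enemy_Shield pawn and runs that pawn's BehaviorShield tree.
; Each AIPerception update scans currently perceived actors and writes the first BP_Character on another team to the Blackboard "Target" key.
; When the scan finds no hostile, it clears that key.
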(event OnPerceptionUpdated(AIPerception)
  (params (UpdatedActors :type Array%20of%20Actor%20Object%20References))
  (CallFunction|Perception))

(event EventPossess
  (params (PossessedPawn :type Pawn%20Object%20Reference))
  (bind _asbp_enemy_shield (Utilities|Casting|CastToBP_Enemy_Shield PossessedPawn))
  (bind _output_get (Variables|Default|SetEnemy_Shield_AI _asbp_enemy_shield))
  (AI|RunBehaviorTree (Variables|/Game/Enemies/Enemy_Shield/BP_Enemy_Shield.BP_Enemy_Shield_C|GetBehavior_Shield _output_get)))

(fn ConstructionScript)

(fn Perception
  (for _array_element (Class|AIPerceptionComponent|GetCurrentlyPerceivedActors (Variables|Default|GetAIPerception))
    (bind _asbp_character (Utilities|Casting|CastToBP_Character _array_element))
    (if (not (Default|IsSameTeam _asbp_character _asbp_character (Variables|Default|GetEnemy_Shield_AI)))
      (AI|Components|Blackboard|SetValueasObject (AI|GetBlackboard 0) (Utilities|Name|MakeLiteralName "Target") _asbp_character)
      (return)))
  (AI|Components|Blackboard|SetValueasObject (AI|GetBlackboard 0) (Utilities|Name|MakeLiteralName "Target") 0))